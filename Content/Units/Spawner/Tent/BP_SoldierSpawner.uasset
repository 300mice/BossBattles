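; Soldier spawner tent that lets the player spawn a unit from warrior data by holding the purchase input nearby.
; InteractRadius overlaps with the player character toggle actor input and show or hide the UnlockMenu widget component.
; While IA_PurchaseUnit is held, elapsed time fills the menu's progress bar against a hardcoded two-second duration.
; On trigger, the unit spawns at SpawnPosition and the bar resets; no cost is checked here.
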(event OnComponentBeginOverlap(InteractRadius)
  (params (OverlappedComponent :type Primitive%20Component%20Object%20Reference) (OtherActor :type Actor%20Object%20Reference) (OtherComp :type Primitive%20Component%20Object%20Reference) (OtherBodyIndex :type Integer) (bFromSweep :type Boolean) (SweepResult :type Hit%20Result%20Structure%20%28by%20ref%29))
  (if (== (Game|GetPlayerCharacter 0) OtherActor)
    (Input|EnableInput (Game|GetPlayerController 0))
    (Rendering|SetVisibility (Variables|Default|GetUnlockMenu) true false)))

(event OnComponentEndOverlap(InteractRadius)
  (params (OverlappedComponent :type Primitive%20Component%20Object%20Reference) (OtherActor :type Actor%20Object%20Reference) (OtherComp :type Primitive%20Component%20Object%20Reference) (OtherBodyIndex :type Integer))
  (if (== (Game|GetPlayerCharacter 0) OtherActor)
    (Input|DisableInput (Game|GetPlayerController 0))
    (Rendering|SetVisibility (Variables|Default|GetUnlockMenu) false false)))

(event Input|EnhancedActionEvents|EnhancedInputActionIA_PurchaseUnit
  (params (ActionValue :type Boolean) (ElapsedSeconds :type Float%20%28double-precision%29) (TriggeredSeconds :type Float%20%28double-precision%29) (InputAction :type Input%20Action%20Object%20Reference :default "/Game/Input/IA_PurchaseUnit.IA_PurchaseUnit"))
  (:Triggered
    (Game|SpawnActorfromClass "/Game/Units/Warrior/WarriorUnit.WarriorUnit_C" (Transformation|GetWorldTransform (Variables|Default|GetSpawnPosition)) "Undefined" "MultiplyWithRoot" 0 "/Game/Units/Warrior/WarriorData.WarriorData" 0)
    (Progress|SetPercent (Variables|/Game/Units/Spawner/Tent/UI_PurchaseUnit_World.UI_PurchaseUnit_World_C|GetUnlockBar (Variables|Default|GetAs%20UI%20Purchase%20Unit%20World)) 0.0))
  (:Started
    (bind _asui_purchase_unit_world (Utilities|Casting|CastToUI_PurchaseUnit_World (UserInterface|GetWidget (Variables|Default|GetUnlockMenu))))
    (Variables|Default|SetAs%20UI%20Purchase%20Unit%20World _asui_purchase_unit_world))
  (:Ongoing
    (Progress|SetPercent (Variables|/Game/Units/Spawner/Tent/UI_PurchaseUnit_World.UI_PurchaseUnit_World_C|GetUnlockBar (Variables|Default|GetAs%20UI%20Purchase%20Unit%20World)) (/ ElapsedSeconds 2.0))))

(event EventBeginPlay
  (Rendering|SetVisibility (Variables|Default|GetUnlockMenu) false false))

(event Collision|EventActorBeginOverlap
  (params (OtherActor :type Actor%20Object%20Reference)))

(event EventTick
  (params (DeltaSeconds :type Float%20%28single-precision%29)))

(fn ConstructionScript)